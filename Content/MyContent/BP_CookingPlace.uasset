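; Cooking station that takes held ingredients from the player and combines them into recipe results.
; CombineIngEvent accepts one of each of five ingredient types, destroys it, sets its flag and shows its indicator.
; Matching trios clear and print No Man Sky, Tears of God or Dead Man's Chest, with other trios giving Shelyxa.
; Only No Man Sky can spawn, gated by HasNoManSky; other spawn branches are hard-wired off.
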(event EventBeginPlay
  (|CallParentFunction) ; This node is disabled and will not be called.\nDrag off pins to build functionality.
)

(event Collision|EventActorBeginOverlap
  (params (OtherActor :type Actor%20Object%20Reference))
  (|CallParentFunction OtherActor) ; This node is disabled and will not be called.\nDrag off pins to build functionality.
)

(event EventTick
  (params (DeltaSeconds :type Float%20%28single-precision%29))
  (|CallParentFunction DeltaSeconds) ; This node is disabled and will not be called.\nDrag off pins to build functionality.
)

(event EventCombineIngEvent
  (params (SecondItem :type Actor%20Object%20Reference) (Player%20REF :type BP%20My%20Main%20Cube%20Object%20Reference))
  (bind _asbp_ingredient_child_sh (Utilities|Casting|CastToBP_IngredientChild_SH SecondItem)
    (:then
      (if (not (Variables|Default|GetbHasSH))
        (Transformation|DetachFromActor _asbp_ingredient_child_sh "KeepWorld" "KeepWorld" "KeepWorld")
        (Variables|/Game/MyContent/BP_MyMainCube.BP_MyMainCube_C|SetHoldingItem Player%20REF 0)
        (Variables|Default|SetbHasSH true)
        (Actor|DestroyActor _asbp_ingredient_child_sh)
        (Rendering|SetVisibility (Variables|Default|GetPlus_SH_Item) true false)
        (Utilities|FlowControl|Sequence
          (:then_0
            (if (Math|Boolean|ANDBoolean (Variables|Default|GetbHasR) (Variables|Default|GetbHasM) (Variables|Default|GetbHasSH)) :!label _label ; No Man Sky
              (Utilities|FlowControl|Sequence
                (:then_0
                  (Variables|Default|SetbHasR false))
                (:then_1
                  (Variables|Default|SetbHasM false))
                (:then_2
                  (Variables|Default|SetbHasSH false)
                  (Rendering|SetVisibility (Variables|Default|GetPlus_SH_Item) false false)
                  (Development|PrintString "NoManSky")
                  (if (not (Variables|Default|GetbHasNoManSky))
                    (Game|SpawnActorfromClass "/Game/MyContent/BP_NoManSky.BP_NoManSky_C" (Math|Transform|MakeTransform (+ (Transformation|GetActorLocation) "0, 0, 0")) "Undefined" 0 0))))))
          (:then_1
            (if (Math|Boolean|ANDBoolean (Variables|Default|GetbHasSH) (Variables|Default|GetbHasA) (Variables|Default|GetbHasVCH)) :!label _label_2 ; Tears Of God
              (Utilities|FlowControl|Sequence
                (:then_0
                  (Variables|Default|SetbHasSH false))
                (:then_1
                  (Variables|Default|SetbHasA false))
                (:then_2
                  (Variables|Default|SetbHasVCH false)
                  (Rendering|SetVisibility (Variables|Default|GetPlus_A_item) false false)
                  (Development|PrintString "TearsOfGod")
                  (if (not true)
                    (Game|SpawnActorfromClass "/Game/MyContent/BP_TearsOfGod.BP_TearsOfGod_C" (Math|Transform|MakeTransform (+ (Transformation|GetActorLocation) "0, 0, 0")) "Undefined" 0 0))))))
          (:then_2
            (if (Math|Boolean|ORBoolean (Math|Boolean|ANDBoolean (Variables|Default|GetbHasA) (Variables|Default|GetbHasM) (Variables|Default|GetbHasVCH)) (Math|Boolean|ANDBoolean (Variables|Default|GetbHasVCH) (Variables|Default|GetbHasM) (Variables|Default|GetbHasSH)) (Math|Boolean|ANDBoolean (Variables|Default|GetbHasR) (Variables|Default|GetbHasA) (Variables|Default|GetbHasVCH)) (Math|Boolean|ANDBoolean (Variables|Default|GetbHasR) (Variables|Default|GetbHasVCH) (Variables|Default|GetbHasSH)) (Math|Boolean|ANDBoolean (Variables|Default|GetbHasR) (Variables|Default|GetbHasVCH) (Variables|Default|GetbHasM)) (Math|Boolean|ANDBoolean (Variables|Default|GetbHasA) (Variables|Default|GetbHasSH) (Variables|Default|GetbHasM))) :!label _label_3
              (Utilities|FlowControl|Sequence
                (:then_0
                  (Variables|Default|SetbHasSH false))
                (:then_1
                  (Variables|Default|SetbHasM false))
                (:then_2
                  (Variables|Default|SetbHasR false))
                (:then_3
                  (Variables|Default|SetbHasA false))
                (:then_4
                  (Variables|Default|SetbHasVCH false)
                  (Rendering|SetVisibility (Variables|Default|GetPlus_A_item) false false)
                  (Development|PrintString "Shelyxa")
                  (if (not true)
                    (Game|SpawnActorfromClass "/Game/MyContent/BP_Shelyxa.BP_Shelyxa_C" (Math|Transform|MakeTransform (+ (Transformation|GetActorLocation) "0, 0, 0")) "Undefined" 0 0)))))))))
    (:CastFailed
      (bind _asbp_ingredient_child_m (Utilities|Casting|CastToBP_IngredientChild_M SecondItem)
        (:then
          (if (not (Variables|Default|GetbHasM))
            (Transformation|DetachFromActor _asbp_ingredient_child_m "KeepWorld" "KeepWorld" "KeepWorld")
            (Variables|/Game/MyContent/BP_MyMainCube.BP_MyMainCube_C|SetHoldingItem Player%20REF 0)
            (Variables|Default|SetbHasM true)
            (Actor|DestroyActor _asbp_ingredient_child_m)
            (Rendering|SetVisibility (Variables|Default|GetPlus_M_Item) true false)
            (Utilities|FlowControl|Sequence
              (:then_0
                (goto _label))
              (:then_1
                (if (Math|Boolean|ANDBoolean (Variables|Default|GetbHasM) (Variables|Default|GetbHasA) (Variables|Default|GetbHasR)) :!label _label_4 ; Dead Mens Chest
                  (Utilities|FlowControl|Sequence
                    (:then_0
                      (Variables|Default|SetbHasM false))
                    (:then_1
                      (Variables|Default|SetbHasA false))
                    (:then_2
                      (Variables|Default|SetbHasR false)
                      (Rendering|SetVisibility (Variables|Default|GetPlus_A_item) false false)
                      (Development|PrintString "DeadMansBody")
                      (if (not true)
                        (Game|SpawnActorfromClass "/Game/MyContent/BP_DeadMansChest.BP_DeadMansChest_C" (Math|Transform|MakeTransform (+ (Transformation|GetActorLocation) "0, 0, 0")) "Undefined" 0 0))))))
              (:then_2
                (goto _label_3)))))
        (:CastFailed
          (bind _asbp_ingredient_child_r (Utilities|Casting|CastToBP_IngredientChild_R SecondItem)
            (:then
              (if (not (Variables|Default|GetbHasR))
                (Transformation|DetachFromActor _asbp_ingredient_child_r "KeepWorld" "KeepWorld" "KeepWorld")
                (Variables|/Game/MyContent/BP_MyMainCube.BP_MyMainCube_C|SetHoldingItem Player%20REF 0)
                (Variables|Default|SetbHasR true)
                (Actor|DestroyActor _asbp_ingredient_child_r)
                (Rendering|SetVisibility (Variables|Default|GetPlus_R_Item) true false)
                (Utilities|FlowControl|Sequence
                  (:then_0
                    (goto _label))
                  (:then_1
                    (goto _label_3))
                  (:then_2
                    (goto _label_4)))))
            (:CastFailed
              (bind _asbp_ingredient_child_a (Utilities|Casting|CastToBP_IngredientChild_A SecondItem)
                (:then
                  (if (not (Variables|Default|GetbHasA))
                    (Transformation|DetachFromActor _asbp_ingredient_child_a "KeepWorld" "KeepWorld" "KeepWorld")
                    (Variables|/Game/MyContent/BP_MyMainCube.BP_MyMainCube_C|SetHoldingItem Player%20REF 0)
                    (Variables|Default|SetbHasA true)
                    (Actor|DestroyActor _asbp_ingredient_child_a)
                    (Rendering|SetVisibility (Variables|Default|GetPlus_A_item) true false)
                    (Utilities|FlowControl|Sequence
                      (:then_0
                        (goto _label_4))
                      (:then_1
                        (goto _label_2))
                      (:then_2
                        (goto _label_3)))))
                (:CastFailed
                  (bind _asbp_ingredient_child_vch (Utilities|Casting|CastToBP_IngredientChild_VCH SecondItem))
                  (if (not (Variables|Default|GetbHasVCH))
                    (Transformation|DetachFromActor _asbp_ingredient_child_vch "KeepWorld" "KeepWorld" "KeepWorld")
                    (Variables|/Game/MyContent/BP_MyMainCube.BP_MyMainCube_C|SetHoldingItem Player%20REF 0)
                    (Variables|Default|SetbHasVCH true)
                    (Actor|DestroyActor _asbp_ingredient_child_vch)
                    (Rendering|SetVisibility (Variables|Default|GetPlus_VCH_Item) true false)
                    (Utilities|FlowControl|Sequence
                      (:then_0
                        (goto _label_2))
                      (:then_1
                        (goto _label_3)))))))))))))

(fn ConstructionScript
  (|CallParentFunction))