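; Player pawn for a timed item-carrying game, moved on world axes with its cube smoothly rotated toward input.
; Tick runs a forward sphere trace, and the PickUp/Drop action passes the hit actor to DeskFunc.
; DeskFunc picks up or places items on a BP_Desk, or combines the held item with a desk's main ingredient.
; A delayed Tick countdown shows the game-over widget and pauses at zero.
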(event EventTick
  (params (DeltaSeconds :type Float%20%28single-precision%29))
  (bind _cube (Variables|Default|GetCube))
  (bind _returnvalue (Transformation|GetWorldLocation _cube))
  (Utilities|FlowControl|Sequence
    (:then_0
      (Utilities|FlowControl|Delay 1.0)
      (if (== (Variables|Default|GetSeconds) 0)
        (if (== (Variables|Default|GetMinutes) 0)
          (bind _returnvalue_2 (UserInterface|CreateWidget "/Game/MyContent/WBP_GameOver.WBP_GameOver_C"))
          (UserInterface|Viewport|AddtoViewport _returnvalue_2 0)
          (Variables|/Script/Engine.PlayerController|SetbShowMouseCursor (Game|GetPlayerController 0) true)
          (Game|SetGamePaused true)
          (else
            (Variables|Default|SetSeconds 59)
            (Variables|Default|SetMinutes (- (Variables|Default|GetMinutes) 1))))
        (else
          (Variables|Default|SetSeconds (- (Variables|Default|GetSeconds) 1)))))
    (:then_1
      (if (or (!= (Input|AxisValues|GetMoveForward) 0.0) (!= (Input|AxisValues|GetMoveRight) 0.0))
        (Variables|Default|SetDirection (Math|Vector|MakeVector (Input|AxisValues|GetMoveForward) (Input|AxisValues|GetMoveRight) 0.0))
        (Transformation|SetWorldRotation (Variables|Default|GetCube) (Math|Rotator|Lerp(Rotator) (Transformation|GetWorldRotation (Variables|Default|GetCube)) (Math|Conversions|RotationFromXVector (Variables|Default|GetDirection)) (* DeltaSeconds (Variables|Default|GetRotationSpeed)) true) false false))
      (bind _outhit (Collision|SphereTraceByChannel _returnvalue (+ _returnvalue (* (Math|Vector|GetForwardVector _cube) (Variables|Default|GetReach))) (Variables|Default|GetRadius) "TraceTypeQuery1" false 0 "ForOneFrame")))))

(event Input|ActionEvents|InputActionPickUp/Drop
  (params (Key :type Key%20Structure :default "None"))
  (:Pressed
    (CallFunction|DeskFunc (.HitActor (Collision|BreakHitResult (stale EventTick _outhit))))))

(event Input|AxisEvents|InputAxisMoveRight
  (params (AxisValue :type Float%20%28single-precision%29))
  (Pawn|Input|AddMovementInput "0.000000,1.000000, 0" AxisValue false))

(event Input|AxisEvents|InputAxisMoveForward
  (params (AxisValue :type Float%20%28single-precision%29))
  (Pawn|Input|AddMovementInput "1.000000,0.000000, 0" AxisValue false))

(fn ConstructionScript)

(fn DeskFunc
  (params (Hit%20Actor :type Actor%20Object%20Reference))
  (bind _asbp_desk (Utilities|Casting|CastToBP_Desk Hit%20Actor))
  (Utilities|IsValid (Variables|/Game/MyContent/BP_Desk.BP_Desk_C|GetItem _asbp_desk)
    (:Is%20Valid
      (Utilities|IsValid (Variables|Default|GetHoldingItem)
        (:Is%20Valid
          (bind _asbp_main_ingredient (Utilities|Casting|CastToBP_MainIngredient (Variables|/Game/MyContent/BP_Desk.BP_Desk_C|GetItem _asbp_desk)))
          (Default|CombineIngEvent _asbp_main_ingredient (Variables|Default|GetHoldingItem) self))
        (:Is%20Not%20Valid
          (Transformation|DetachFromActor (Variables|/Game/MyContent/BP_Desk.BP_Desk_C|GetItem _asbp_desk) "KeepWorld" "KeepWorld" "KeepWorld")
          (bind _output_get (Variables|Default|SetHoldingItem (Variables|/Game/MyContent/BP_Desk.BP_Desk_C|GetItem _asbp_desk)))
          (Transformation|AttachComponentToComponent _output_get (Variables|Default|GetHoldingItemLocation) "None" "SnapToTarget" "KeepWorld" "KeepWorld" true)
          (Variables|/Game/MyContent/BP_Desk.BP_Desk_C|SetItem _asbp_desk 0))))
    (:Is%20Not%20Valid
      (Utilities|IsValid (Variables|Default|GetHoldingItem)
        (:Is%20Valid
          (Transformation|DetachFromActor (Variables|Default|GetHoldingItem) "KeepWorld" "KeepWorld" "KeepWorld")
          (Transformation|AttachComponentToComponent (Variables|Default|GetHoldingItem) (Variables|/Game/MyContent/BP_Desk.BP_Desk_C|GetItemLocation _asbp_desk) "None" "SnapToTarget" "KeepWorld" "KeepWorld" true)
          (Variables|/Game/MyContent/BP_Desk.BP_Desk_C|SetItem _asbp_desk (Variables|Default|GetHoldingItem))
          (Variables|Default|SetHoldingItem 0))))))